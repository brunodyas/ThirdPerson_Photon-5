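; Photon Cloud networking Blueprint that connects a third-person game to a multiplayer room and spawns its players.
; Once the controller is ready, a delayed init connects under a GUID name and joins or creates one of two rooms, chosen by a map flag.
; A timer moves the local pawn to a random player start.
; The local player's join sets up its pawn, while remote joins spawn character replicas at random starts.
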(event `On Controller Is Ready`
  (params (`3rd Player Controler ` :type "/Game/ThirdPersonBP/Blueprints/ThirdPersonController Object Reference"))
  (set `self.LocalController` `3rd Player Controler `)
  (`KismetSystemLibrary.K2_SetTimerDelegate` (delegate `Init Game`) 1.0))

(event `Init Game`
  ;[1 1 1] cache
  (if (not (`self.bGameInitialized`))
    (set `self.bGameInitialized` true)
    (set `self.PlayerStarts` (`/Game/ThirdPersonBP/Blueprints/ThirdPersonController.GetPlayerStarts` (`self.LocalController`)))
    ;[1 1 1] Connect
    (add `self.OnPhotonCloudConnected` (delegate `On Connect`))
    (add `self.OnPlayerJoinedRoom` (delegate `On Player Joined`))
    (`self.SetPlayerName` (`KismetGuidLibrary.Conv_GuidToString` (`KismetGuidLibrary.NewGuid`)))
    (`self.Connect`)
    (`KismetSystemLibrary.K2_SetTimerDelegate` (delegate `First Location of the player`) 2.0)))

(event `First Location of the player`
  (bind _playerstarts (`self.PlayerStarts`))
  ;[1 1 1] Connect
  (`Actor.K2_SetActorLocation` (`Controller.K2_GetPawn` (`self.LocalController`)) (`Actor.K2_GetActorLocation` (`|GetArrayItem` _playerstarts (`KismetMathLibrary.RandomIntegerInRange` 0 (`KismetArrayLibrary.Array_LastIndex` _playerstarts)))) false false))

(event `On Connect`
  ;[1 1 1] Connect
  (if (`self.bGameGotoMap`)
    (`self.JoinOrCreateRoom` "SalaMapa2" 10 null)
    (else
      (`self.JoinOrCreateRoom` "thirdpersontest" 10 null))))

(event `On Player Joined` :!signature `self.OnPlayerJoinedRoom`
  (params (PlayerNumber :type Integer) (PlayerName :type String) (IsLocalPlayer :type Boolean))
  (bind _playerstarts (`self.PlayerStarts`))
  (bind (_returnvalue_location _returnvalue_rotation) (`KismetMathLibrary.BreakTransform` (`Actor.GetTransform` (`|GetArrayItem` _playerstarts (`KismetMathLibrary.RandomIntegerInRange` 0 (- (`KismetArrayLibrary.Array_Length` _playerstarts) 1))))))
  ;[1 1 1] Join a room
  (if IsLocalPlayer
    (`/Game/ThirdPersonBP/Blueprints/ThirdPersonCharacter.Setup Player` (cast `/Game/ThirdPersonBP/Blueprints/ThirdPersonCharacter` (`Controller.K2_GetPawn` (`self.LocalController`)) :!pure true) PlayerNumber self)
    (else
      (bind _characterreplica (`/Game/ThirdPersonBP/Blueprints/ThirdPersonController.CreateCharacterReplica` (`self.LocalController`) (`KismetMathLibrary.MakeTransform` _returnvalue_location _returnvalue_rotation)))
      (`/Game/ThirdPersonBP/Blueprints/ThirdPersonCharacter.Setup Player` _characterreplica PlayerNumber self))))

(fn `UserConstructionScript`)